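; AI controller that walks its controlled Ai_Character along a chain of linked path nodes.
; On BeginPlay it caches the pawn and moves it to the pawn's DesiredNode.
; Each tick, if the move status differs from DesiredStatus, it advances DesiredNode to its NextNode.
; It then issues a move to the node after the new DesiredNode, so the target sits one link ahead of the stored node.
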(event `self.ReceiveBeginPlay`
  (bind _asai_character (cast `/Game/BluePrints/Ai/Ai_Character` (`self.K2_GetPawn`)))
  (bind _output_get (set `self.Stored Pawn` _asai_character))
  (`self.MoveToActor` (`/Game/BluePrints/Ai/Ai_Character.DesiredNode` _output_get) 1.0))

(event `self.ReceiveTick`
  (params (DeltaSeconds :type "Float (single-precision)"))
  (bind _stored_pawn (`self.Stored Pawn`))
  (bind _nextnode (`/Game/BluePrints/AI_Helpers/PathNode.NextNode` (`/Game/BluePrints/Ai/Ai_Character.DesiredNode` _stored_pawn)))
  (if (!= (`self.GetMoveStatus`) (`self.DesiredStatus`))
    (set `/Game/BluePrints/Ai/Ai_Character.DesiredNode` _nextnode _stored_pawn)
    (`self.MoveToActor` _nextnode 1.0)))

(fn `UserConstructionScript`)