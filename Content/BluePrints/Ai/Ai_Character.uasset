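; AI character that patrols a chain of PathNode actors and moves toward a pawn it sees.
; BeginPlay starts movement at DesiredNode; each node overlap sets walk speed and sends it to that node's NextNode.
; PawnSensing latches InRange and starts a chase, which Tick tries to repeat, though its target cast is never executed.
; HandleHitByGun destroys the character unless it is stunned.
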(event OnSeePawn(PawnSensing)
  (params (Pawn :type Pawn%20Object%20Reference))
  (Variables|Default|SetInRange true)
  (bind _asthird_person_character (Utilities|Casting|CastToThirdPersonCharacter Pawn))
  (AI|AIMoveTo self "0, 0, 0" _asthird_person_character 5.0 false))

(event EventTick
  (params (DeltaSeconds :type Float%20%28single-precision%29))
  (if (Variables|Default|GetInRange)
    (if (not (Variables|Default|Getmoving))
      (AI|AIMoveTo self "0, 0, 0" (stale _asthird_person_character) 5.0 false
        (:then
          (Variables|Default|Setmoving true)
          (if (Variables|Default|GetInRange)
            _))
        (:OnSuccess
          (Variables|Default|Setmoving false :!label _label))
        (:OnFail
          (goto _label))))))

(event Collision|EventActorBeginOverlap
  (params (OtherActor :type Actor%20Object%20Reference))
  (bind _aspath_node (Utilities|Casting|CastToPathNode OtherActor))
  (Variables|/Script/Engine.CharacterMovementComponent|SetMaxWalkSpeed (Variables|Character|GetCharacterMovement) (Variables|/Game/BluePrints/AI_Helpers/PathNode.PathNode_C|GetWalkSpeed _aspath_node))
  (AI|Navigation|MovetoActor (stale EventBeginPlay _asaicontroller) (Variables|/Game/BluePrints/AI_Helpers/PathNode.PathNode_C|GetNextNode _aspath_node) 1.0 true true))

(event EventBeginPlay
  (Pawn|SpawnDefaultController)
  (bind _asaicontroller (Utilities|Casting|CastToAIController (Pawn|GetController)))
  (bind _returnvalue (AI|Navigation|MovetoActor _asaicontroller (Variables|Default|GetDesiredNode) 1.0 true true))
  (if (!= (Class|AIController|GetMoveStatus _asaicontroller) _returnvalue)
    (Variables|Default|SetDesiredNode (Variables|/Game/BluePrints/AI_Helpers/PathNode.PathNode_C|GetNextNode (Variables|Default|GetDesiredNode)))
    (AI|Navigation|MovetoActor _asaicontroller (Variables|/Game/BluePrints/AI_Helpers/PathNode.PathNode_C|GetNextNode (Variables|Default|GetDesiredNode)) 1.0 true true)))

(fn ConstructionScript)

(fn HandleHitbyGun
  (if (not (Variables|Default|GetIsStunned))
    (Actor|DestroyActor)))